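; BP_Simulation is a molecular simulation actor that sets up and steps a simulation cell with optional solvent and molecules.
; BeginPlay builds the cell, applies the solvent modifier, spawns configured molecules, then applies debug display toggles for center of mass, collision and interaction spheres, splines, and a render style.
; Tick calls UpdateSimulation every frame, while an ActivateSimulation call is left unconnected.
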(event EventBeginPlay
  (Class|Simulation|InitSimulationCell (Variables|Simulation|GetSimulationCellWidth) (Math|Color|MakeColor 255 255 0 255) (Variables|Simulation|GetbTeleportWalls))
  (Class|Simulation|InitSimulation)
  (Class|Simulation|SetSolventModifier (Variables|Simulation|GetCurrentSolventModifier))
  (if (Variables|Simulation|GetbAddSolvent)
    (Class|Simulation|InitSolvent (Variables|Simulation|GetSolventName)))
  (if (Variables|Simulation|GetbSpawnNumMolecules)
    (Class|Simulation|InitNumMolecules (Variables|Simulation|GetMoleculeName) (Variables|Simulation|GetNumMolecules)))
  (if (Variables|Simulation|GetbShowCoM)
    (Class|Simulation|SetShowCoM)
    (else
      (Class|Simulation|SetHideCoM)))
  (if (Variables|Simulation|GetShowCollision)
    (Class|Simulation|SetShowCollisionSpheres)
    (else
      (Class|Simulation|SetHideCollisionSpheres)))
  (if (Variables|Simulation|GetbShowInteractionSphere)
    (Class|Simulation|SetShowInteractionSpheres)
    (else
      (Class|Simulation|SetHideInteractionSpheres)))
  (if (Variables|Simulation|GetbShowSplines)
    (Class|Simulation|SetShowSpline)
    (else
      (Class|Simulation|SetHideSpline)))
  (switch int (Variables|Simulation|GetRenderStyle)
    (:Default
      (Class|Simulation|SetRenderBallStick :!label _label))
    (:0
      (Class|Simulation|SetRenderHidden))
    (:1
      (Class|Simulation|SetRenderLinear))
    (:2
      (goto _label))
    (:3
      (Class|Simulation|SetRenderSpaceFilling)))
  (Utilities|FlowControl|Delay 0.5))

(event EventTick
  (params (DeltaSeconds :type Float%20%28single-precision%29))
  (Class|Simulation|UpdateSimulation))

(fn ConstructionScript)